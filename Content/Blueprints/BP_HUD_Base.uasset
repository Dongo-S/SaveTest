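; Base HUD that manages an exit-confirmation menu and an instructions overlay.
; On BeginPlay it creates both widgets, adds them to the viewport and passes itself to the exit widget.
; The OpenExit event calls ToggleExitQuestion, which swaps which widget is shown and switches the mouse cursor and input mode between game-only and UI-only focused on the menu.
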(event `self.ReceiveBeginPlay`
  (bind _returnvalue (`|CreateWidget` "/Game/Widgets/Widget_ExitMenu.Widget_ExitMenu_C" (`self.GetOwningPlayerController`)))
  (bind _output_get (set `self.WG_Exit` _returnvalue))
  (`UserWidget.AddToViewport` _output_get 0)
  (`/Game/Widgets/Widget_ExitMenu.SetHUDBase` _output_get self)
  (bind _returnvalue_2 (`|CreateWidget` "/Game/Widgets/Widget_Instructions.Widget_Instructions_C" (`self.GetOwningPlayerController`)))
  (bind _output_get_2 (set `self.WG_Instructions` _returnvalue_2))
  (`UserWidget.AddToViewport` _output_get_2 0))

(event `OpenExit`
  (`self.ToggleExitQuestion`))

(fn `ToggleExitQuestion`
  (bind _returnvalue (`self.GetOwningPlayerController`))
  (bind _wg_exit (`self.WG_Exit`))
  (bind _wg_instructions (`self.WG_Instructions`))
  (if (`Widget.IsVisible` _wg_exit)
    (`Widget.SetVisibility` _wg_exit "Collapsed")
    (`Widget.SetVisibility` _wg_instructions "Visible")
    (set `PlayerController.bShowMouseCursor` false _returnvalue)
    (`WidgetBlueprintLibrary.SetInputMode_GameOnly` _returnvalue)
    (else
      (`Widget.SetVisibility` _wg_exit "Visible")
      (`Widget.SetVisibility` _wg_instructions "Collapsed")
      (set `PlayerController.bShowMouseCursor` true _returnvalue)
      (`WidgetBlueprintLibrary.SetInputMode_UIOnlyEx` _returnvalue (`self.WG_Exit`)))))

(fn `UserConstructionScript`)